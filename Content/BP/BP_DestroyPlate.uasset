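; BP_DestroyPlate is a platform that falls away after the third-person character steps into its Box trigger.
; After a Lifetime delay, MoveComponentTo drops the Cube far down over one second, then the Cube is hidden and loses collision.
; A Respawn event, not called within this Blueprint, restores visibility and collision and moves the Cube back to its relative origin.
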(event OnComponentBeginOverlap(Box)
  (params (OverlappedComponent :type Primitive%20Component%20Object%20Reference) (OtherActor :type Actor%20Object%20Reference) (OtherComp :type Primitive%20Component%20Object%20Reference) (OtherBodyIndex :type Integer) (bFromSweep :type Boolean) (SweepResult :type Hit%20Result%20Structure%20%28by%20ref%29))
  (Utilities|Casting|CastToBP_ThirdPersonCharacter OtherActor)
  (Utilities|FlowControl|Delay (Variables|Default|GetLifetime))
  (Components|MoveComponentTo (Variables|Default|GetCube) "0.000000,0.000000,-2150.000000" "0, 0, 0" false false 1.0 false)
  (Rendering|SetVisibility (Variables|Default|GetCube) false false)
  (Collision|SetCollisionEnabled (Variables|Default|GetCube) "NoCollision"))

(event Custom|Respawn
  (Rendering|SetVisibility (Variables|Default|GetCube) true false)
  (Collision|SetCollisionEnabled (Variables|Default|GetCube) "QueryAndPhysics")
  (Components|MoveComponentTo (Variables|Default|GetCube) "0, 0, 0" "0, 0, 0" false false 1.0 false))

(event EventBeginPlay)

(event Collision|EventActorBeginOverlap
  (params (OtherActor :type Actor%20Object%20Reference)))

(event EventTick
  (params (DeltaSeconds :type Float%20%28single-precision%29)))

(fn ConstructionScript)