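; Enemy actor that wanders around its spawn point and damages the player on contact.
; BeginPlay stores the start location and starts an endless patrol loop: AI MoveTo a random reachable point, then a random delay.
; The delay hangs off MoveTo's immediate output, so new moves don't wait for arrival.
; Sphere overlap with BP_ThirdPersonCharacter applies damage to player character 0 after a short delay.
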(event OnComponentBeginOverlap(Sphere)
  (params (OverlappedComponent :type Primitive%20Component%20Object%20Reference) (OtherActor :type Actor%20Object%20Reference) (OtherComp :type Primitive%20Component%20Object%20Reference) (OtherBodyIndex :type Integer) (bFromSweep :type Boolean) (SweepResult :type Hit%20Result%20Structure%20%28by%20ref%29))
  ;[1 1 1] Damage
  (Utilities|Casting|CastToBP_ThirdPersonCharacter OtherActor)
  (Utilities|FlowControl|Delay 0.1)
  (Game|Damage|ApplyDamage (Game|GetPlayerCharacter 0) (Variables|Default|GetBase%20Damage) 0 0))

(event Custom|StartPatrolling
  ;[1 1 1] Patrol
  (if true :!label _label
    (AI|AIMoveTo self (.RandomLocation (AI|Navigation|GetRandomReachablePointinRadius (Variables|Default|GetStartingLocation) (Variables|Default|GetPatrolRadius) 0 0)) 0 2e+01 false
      (:then
        (Utilities|FlowControl|Delay (Math|Random|RandomFloatinRange (Variables|Default|GetPatrolDelayMin) (Variables|Default|GetPatrolDelayMax)))
        (goto _label)))))

(event EventBeginPlay
  ;[1 1 1] BeginPlay
  (Variables|Default|SetStartingLocation (Transformation|GetActorLocation))
  (CallFunction|StartPatrolling))

(event Collision|EventActorBeginOverlap
  (params (OtherActor :type Actor%20Object%20Reference)))

(event EventTick
  (params (DeltaSeconds :type Float%20%28single-precision%29)))

(fn ConstructionScript)